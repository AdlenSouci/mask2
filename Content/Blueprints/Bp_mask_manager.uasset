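; Mask manager that switches the player's active mask between blue, green and red variants.
; BeginPlay caches the Masky player controller, the post-process actor and the player's Masky pawn.
; MaskSwitch sets the current mask, applies the matching post-process filter and mesh material, then calls the controller's mask-change dispatcher.
; Each switch locks further switching until a cooldown timer re-enables it.
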(event Custom|Activate_switch
  (Variables|Default|SetCan_switch true))

(event Custom|Desactivate_switch
  (Variables|Default|SetCan_switch false)
  (Utilities|Time|SetTimerbyEvent (delegate Custom|Activate_switch) (Variables|Default|GetCooldown) false true))

(event EventBeginPlay
  (bind _asbp_player_controller_masky (Utilities|Casting|CastToBP_Player_Controller_Masky (Game|GetPlayerController 0)))
  (Variables|Default|Set%20BP%20Player%20Controller%20ref _asbp_player_controller_masky)
  (bind _returnvalue (Actor|GetActorOfClass "/Game/Blueprints/Elements/BP_PostProcess.BP_PostProcess_C"))
  (Variables|Default|SetFilter _returnvalue)
  (bind _asbp_masky (Utilities|Casting|CastToBP_Masky (Game|Player|GetPlayerPawn 0)))
  (Variables|Default|SetAs%20BP%20Masky _asbp_masky))

(fn ConstructionScript)

(fn MaskSwitch
  (params (Mask_value :type Integer))
  (bind __bp_player_controller_ref (Variables|Default|Get%20BP%20Player%20Controller%20ref))
  (if (Variables|Default|GetCan_switch)
    (switch int Mask_value
      (:1
        (Variables|Default|SetCurrent_mask "NewEnumerator0")
        (Default|Blue (Variables|Default|GetFilter))
        (Rendering|Material|SetMaterial (Variables|/Script/Engine.Character|GetMesh (Variables|Default|GetAs%20BP%20Masky)) 10 "/Game/Assets/Character/Blue.Blue")
        (Default|CallEDMaskChange __bp_player_controller_ref))
      (:2
        (Variables|Default|SetCurrent_mask "NewEnumerator1")
        (Default|Green (Variables|Default|GetFilter))
        (Rendering|Material|SetMaterial (Variables|/Script/Engine.Character|GetMesh (Variables|Default|GetAs%20BP%20Masky)) 10 "/Game/Assets/Character/Green.Green")
        (Default|CallEDMaskChange __bp_player_controller_ref))
      (:3
        (Variables|Default|SetCurrent_mask "NewEnumerator2")
        (Default|Red (Variables|Default|GetFilter))
        (Rendering|Material|SetMaterial (Variables|/Script/Engine.Character|GetMesh (Variables|Default|GetAs%20BP%20Masky)) 10 "/Game/Assets/Character/M_Glass_Character.M_Glass_Character")
        (Default|CallEDMaskChange __bp_player_controller_ref)))
    (CallFunction|DesactivateSwitch)))
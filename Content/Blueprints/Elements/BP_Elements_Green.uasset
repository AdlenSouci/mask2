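; Green element Blueprint that appears only while the green mask is the current mask.
; On BeginPlay it binds to the player controller's mask-change dispatcher and checks the mask manager's current mask.
; Green unhides the actor and sets only the test box to query-only collision.
; Blue or Red hides it and disables collision on both the real platform and the test box.
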(event Custom|Green_Mask_management
  (switch Utilities|FlowControl|Switch|SwitchonEnum_mask (Variables|/Game/Blueprints/Bp_mask_manager.Bp_mask_manager_C|GetCurrent_mask (Variables|Default|GetMask_manager_ref))
    (:NewEnumerator0
      (CallFunction|DesaffichageElementsGreens :!label _label))
    (:NewEnumerator1
      (CallFunction|AffichageElementsGreen))
    (:NewEnumerator2
      (goto _label))))

(event EventBeginPlay
  (|CallParentFunction)
  (EventDispatchers|BindEventtoEDMaskChange (Variables|Default|GetPlayer_controller_ref) (delegate Custom|Green_Mask_management)))

(event Collision|EventActorBeginOverlap
  (params (OtherActor :type Actor%20Object%20Reference)))

(event EventTick
  (params (DeltaSeconds :type Float%20%28single-precision%29))
  (|CallParentFunction DeltaSeconds))

(fn ConstructionScript
  (|CallParentFunction))

(fn AffichageElementsGreen
  (Rendering|SetActorHiddenInGame false)
  (Collision|SetCollisionEnabled (Variables|Default|GetBox_plateforme_test_collision) "QueryOnly"))

(fn DesaffichageElementsGreens
  (Rendering|SetActorHiddenInGame true)
  (Collision|SetCollisionEnabled (Variables|Default|Getplateforme_reel) "NoCollision"))
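; BP_check_point is a checkpoint trigger that saves a position when BP_Masky enters its capsule.
; On overlap it shows a widget, plays its checkpoint animation and sound, then disables capsule collision so it fires once.
; It stores its raised X/Z position, with the controller's Y, plus the BP_Fog actor's X location on BP_Player_Controller_Masky.
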(event OnComponentBeginOverlap(Capsule)
  (params (OverlappedComponent :type Primitive%20Component%20Object%20Reference) (OtherActor :type Actor%20Object%20Reference) (OtherComp :type Primitive%20Component%20Object%20Reference) (OtherBodyIndex :type Integer) (bFromSweep :type Boolean) (SweepResult :type Hit%20Result%20Structure%20%28by%20ref%29))
  (bind _returnvalue (Transformation|GetActorLocation))
  (bind _widget (Variables|Default|GetWidget))
  (bind _controller_ref (Variables|Default|GetController_ref))
  (Utilities|Casting|CastToBP_Masky OtherActor
    (:then
      (Rendering|SetVisibility _widget true false)
      (bind _asui_checkpoint (Utilities|Casting|CastToUI_checkpoint (UserInterface|GetWidget _widget)))
      (UserInterface|Animation|PlayAnimation _asui_checkpoint (Variables|/Game/Blueprints/UI/widget/UI_checkpoint.UI_checkpoint_C|Getanim_check_point _asui_checkpoint) 0.0 1 "Forward" 1.0 false)
      (Default|StartCheckpointSound (Variables|Default|Getsound_ref))
      (Collision|SetCollisionEnabled (Variables|Default|GetCapsule) "NoCollision")
      (Variables|/Game/Blueprints/BP_Player_Controller_Masky.BP_Player_Controller_Masky_C|SetPlayer_coordinante_check_point _controller_ref (Math|Vector|MakeVector (.x _returnvalue) (.y (Transformation|GetActorLocation _controller_ref)) (+ (.z _returnvalue) 1.2e+02)))
      (bind _returnvalue_2 (Actor|GetActorOfClass "/Game/Blueprints/Elements/BP_Fog.BP_Fog_C"))
      (Variables|/Game/Blueprints/BP_Player_Controller_Masky.BP_Player_Controller_Masky_C|SetFog_X_Location (Variables|Default|GetController_ref) (.x (Transformation|GetActorLocation _returnvalue_2))))
    (:CastFailed
      (Development|PrintString "Hello"))))

(event EventBeginPlay
  (bind _asbp_player_controller_masky (Utilities|Casting|CastToBP_Player_Controller_Masky (Game|GetPlayerController 0)))
  (Variables|Default|SetController_ref _asbp_player_controller_masky)
  (bind _returnvalue (Actor|GetActorOfClass "/Game/Blueprints/BP_Sound_Controller.BP_Sound_Controller_C"))
  (Variables|Default|Setsound_ref _returnvalue))

(event Collision|EventActorBeginOverlap
  (params (OtherActor :type Actor%20Object%20Reference)))

(event EventTick
  (params (DeltaSeconds :type Float%20%28single-precision%29)))

(fn ConstructionScript)
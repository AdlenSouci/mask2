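; Trigger volume actor that speeds up and repositions the gas fog (BP_Fog), which it looks up on BeginPlay.
; When the fog overlaps the box, the trigger calls AccelerateFog on it and stays in the level.
; When BP_Masky overlaps it, the trigger also accelerates the fog, moves it to a fixed offset back along world X from itself, then destroys itself.
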(event OnComponentBeginOverlap(Box)
  (params (OverlappedComponent :type Primitive%20Component%20Object%20Reference) (OtherActor :type Actor%20Object%20Reference) (OtherComp :type Primitive%20Component%20Object%20Reference) (OtherBodyIndex :type Integer) (bFromSweep :type Boolean) (SweepResult :type Hit%20Result%20Structure%20%28by%20ref%29))
  (bind _returnvalue (Transformation|GetActorLocation))
  (bind _gaz_ref (Variables|Default|GetGaz_ref))
  (if (== OtherActor (Variables|Default|GetGaz_ref))
    (Default|AccelerateFog _gaz_ref)
    (else
      (Utilities|Casting|CastToBP_Masky OtherActor)
      (Default|AccelerateFog (Variables|Default|GetGaz_ref))
      (Transformation|SetActorLocation _gaz_ref (Math|Vector|MakeVector (- (.x _returnvalue) 1.5e+03) (.y _returnvalue) 0.0) false false)
      (Actor|DestroyActor))))

(event EventBeginPlay
  (bind _returnvalue (Actor|GetActorOfClass "/Game/Blueprints/Elements/BP_Fog.BP_Fog_C"))
  (Variables|Default|SetGaz_ref _returnvalue))

(fn ConstructionScript)
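; BP_Victory is a goal trigger actor that ends a level in victory when the player character BP_Masky reaches it.
; On BeginPlay it finds the level's Timer actor and adds a W_Victory widget to the viewport.
; When BP_Masky overlaps its Box, it pauses the timer and calls Victory on that widget.
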(event OnComponentBeginOverlap(Box)
  (params (OverlappedComponent :type Primitive%20Component%20Object%20Reference) (OtherActor :type Actor%20Object%20Reference) (OtherComp :type Primitive%20Component%20Object%20Reference) (OtherBodyIndex :type Integer) (bFromSweep :type Boolean) (SweepResult :type Hit%20Result%20Structure%20%28by%20ref%29))
  (Utilities|Casting|CastToBP_Masky OtherActor)
  (Default|PauseTimer (Variables|Default|Gettimer_ref))
  (Default|Victory (Variables|Default|GetVictory%20Widget)))

(event EventBeginPlay
  (bind _returnvalue (Actor|GetActorOfClass "/Game/Blueprints/Timer.Timer_C"))
  (Variables|Default|Settimer_ref _returnvalue)
  (bind _returnvalue_2 (UserInterface|CreateWidget "/Game/Blueprints/UI/widget/W_Victory.W_Victory_C"))
  (bind _output_get (Variables|Default|SetVictory%20Widget _returnvalue_2))
  (UserInterface|Viewport|AddtoViewport _output_get 0))

(fn ConstructionScript)
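; BP_Elements_Red is a red world element that turns passable while the player's current mask is Red.
; On BeginPlay it calls its parent, then binds a handler to the player controller's mask-change event dispatcher.
; The handler reads the mask manager's current mask and makes the cube translucent without collision for Red, or opaque red with full collision for Blue or Green.
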(event Custom|Red_Mask_Management
  ;[1 1 1] Gère la gestion du red Mask Management
  (switch Utilities|FlowControl|Switch|SwitchonEnum_mask (Variables|/Game/Blueprints/Bp_mask_manager.Bp_mask_manager_C|GetCurrent_mask (Variables|Default|GetMask_manager_ref))
    (:NewEnumerator0
      (Rendering|Material|SetMaterial (Variables|Default|GetCube) 0 "/Game/Materials/Material_Instance/MI_Red.MI_Red" :!label _label)
      (Collision|SetCollisionEnabled (Variables|Default|GetCube) "QueryAndPhysics"))
    (:NewEnumerator1
      (goto _label))
    (:NewEnumerator2
      (Rendering|Material|SetMaterial (Variables|Default|GetCube) 0 "/Game/Materials/Material_Instance/MI_RedTranslucent.MI_RedTranslucent")
      (Collision|SetCollisionEnabled (Variables|Default|GetCube) "NoCollision"))))

(event EventBeginPlay
  ;[1 1 1] Gère la gestion du red Mask Management
  (|CallParentFunction)
  (EventDispatchers|BindEventtoEDMaskChange (Variables|Default|GetPlayer_controller_ref) (delegate Custom|Red_Mask_Management)))

(fn ConstructionScript
  (|CallParentFunction))
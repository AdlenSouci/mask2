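; BP_Fog is an advancing fog hazard that drains BP_Masky's oxygen while the player overlaps its box.
; Tick moves it along local X by base speed and a multiplier, which AccelerateFog compounds.
; A Delay in Tick throttles the drain; at zero oxygen it reloads Lv1, or restores player and fog from checkpoint data stored on the controller.
; Overlap events switch BP_Sound_Controller between global and fog music.
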(event OnComponentBeginOverlap(Box)
  (params (OverlappedComponent :type Primitive%20Component%20Object%20Reference) (OtherActor :type Actor%20Object%20Reference) (OtherComp :type Primitive%20Component%20Object%20Reference) (OtherBodyIndex :type Integer) (bFromSweep :type Boolean) (SweepResult :type Hit%20Result%20Structure%20%28by%20ref%29))
  (bind _sound_ref (Variables|Default|Getsound_ref))
  (bind _sound_ref_2 (Variables|Default|Getsound_ref))
  (bind _asbp_masky (Utilities|Casting|CastToBP_Masky OtherActor))
  (Variables|Default|SetPlayer _asbp_masky)
  (Variables|Default|SetDecreaseOxygene true)
  (Utilities|IsValid _sound_ref_2
    (:Is%20Valid
      (Default|PauseGlobalMusic _sound_ref_2)
      (Utilities|IsValid _sound_ref
        (:Is%20Valid
          (Default|StartFogMusic _sound_ref))))))

(event OnComponentEndOverlap(Box)
  (params (OverlappedComponent :type Primitive%20Component%20Object%20Reference) (OtherActor :type Actor%20Object%20Reference) (OtherComp :type Primitive%20Component%20Object%20Reference) (OtherBodyIndex :type Integer))
  (bind _sound_ref (Variables|Default|Getsound_ref))
  (bind _sound_ref_2 (Variables|Default|Getsound_ref))
  (Utilities|Casting|CastToBP_Masky OtherActor)
  (Variables|Default|SetDecreaseOxygene false)
  (Utilities|IsValid _sound_ref_2
    (:Is%20Valid
      (Default|PauseFogMusic _sound_ref_2)
      (Utilities|IsValid _sound_ref
        (:Is%20Valid
          (Default|StartGlobalMusic _sound_ref))))))

(event EventBeginPlay
  (bind _returnvalue (Actor|GetActorOfClass "/Game/Blueprints/BP_Sound_Controller.BP_Sound_Controller_C"))
  (bind _output_get (Variables|Default|Setsound_ref _returnvalue))
  (Default|PauseFogMusic _output_get))

(event EventTick
  (params (DeltaSeconds :type Float%20%28single-precision%29))
  (bind _returnvalue (Transformation|GetActorLocation))
  (bind _basespeed (Variables|Default|GetBaseSpeed))
  (bind _multiplier (Variables|Default|GetMultiplier))
  (bind _returnvalue_2 (* _basespeed _multiplier DeltaSeconds))
  (Utilities|FlowControl|Sequence
    (:then_0
      (Development|PrintString (Utilities|String|ToString(Float) _returnvalue_2) true true "(R=0.000000,G=0.660000,B=1.000000,A=1.000000)" 0.0)
      (Transformation|AddActorLocalOffset (Math|Vector|MakeVector _returnvalue_2 0.0 0.0) false false))
    (:then_1
      (if (Variables|Default|GetDecreaseOxygene)
        (Utilities|FlowControl|Delay 0.05)
        (bind _result (Math|Integer|DecrementInt (Variables|/Game/Blueprints/BP_Masky.BP_Masky_C|GetOxygene (Variables|Default|GetPlayer)))
          (:%20%20
            (if (<= _result 0)
              (if (== (.x (Variables|/Game/Blueprints/BP_Player_Controller_Masky.BP_Player_Controller_Masky_C|GetPlayer_coordinante_check_point (Variables|/Game/Blueprints/BP_Masky.BP_Masky_C|GetControllerRef (Variables|Default|GetPlayer)))) 0.0)
                (Game|OpenLevel(byName) "Lv1")
                (else
                  (Variables|/Game/Blueprints/BP_Masky.BP_Masky_C|SetOxygene (Variables|Default|GetPlayer) 100)
                  (Transformation|SetActorLocation (Variables|Default|GetPlayer) (Variables|/Game/Blueprints/BP_Player_Controller_Masky.BP_Player_Controller_Masky_C|GetPlayer_coordinante_check_point (Variables|/Game/Blueprints/BP_Masky.BP_Masky_C|GetControllerRef (Variables|Default|GetPlayer))) false true)
                  (Transformation|SetActorLocation (Math|Vector|MakeVector (Variables|/Game/Blueprints/BP_Player_Controller_Masky.BP_Player_Controller_Masky_C|GetFog_X_Location (Variables|/Game/Blueprints/BP_Masky.BP_Masky_C|GetControllerRef (Variables|Default|GetPlayer))) (.y _returnvalue) (.z _returnvalue)) false false))))))))))

(fn ConstructionScript)

(fn AccelerateFog
  (Variables|Default|SetMultiplier (* (Variables|Default|GetMultiplier) (Variables|Default|GetMultiplierStep))))
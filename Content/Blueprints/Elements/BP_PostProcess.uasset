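; BP_PostProcess is a Blueprint that switches the color cast of its PostProcess component between three presets.
; Custom events Blue, Green and Red each assign new post-process settings with a different white balance temperature and tint.
; Each event replaces the whole Settings struct instantly, with no blending, and the construction script is empty.
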(event Custom|Red
  (Variables|/Script/Engine.PostProcessComponent|SetSettings (Variables|Default|GetPostProcess) (Utilities|Struct|MakePostProcessSettings 1.5e+04 1.0)))

(event Custom|Blue
  (Variables|/Script/Engine.PostProcessComponent|SetSettings (Variables|Default|GetPostProcess) (Utilities|Struct|MakePostProcessSettings 6.5e+03)))

(event Custom|Green
  (Variables|/Script/Engine.PostProcessComponent|SetSettings (Variables|Default|GetPostProcess) (Utilities|Struct|MakePostProcessSettings 1.5e+04 -0.9)))

(fn ConstructionScript)
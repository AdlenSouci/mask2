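; BP_Timer is a timer Blueprint that counts elapsed minutes and seconds from BeginPlay.
; StartTimer stores the handle of a looping one-second timer, which PauseTimer can pause.
; Each tick calls TimeCalcule, which increments seconds, rolls over to the next minute only after seconds reach 60, and returns formatted text.
; The timer event itself discards that returned text.
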(event Custom|StartTimer
  (bind _returnvalue (Utilities|Time|SetTimerbyEvent (delegate Custom|Deta1Second) 1.0 true))
  (Variables|Default|SetTimer _returnvalue))

(event Custom|Deta1Second
  (CallFunction|TimeCalcule))

(event Custom|Pause%20Timer
  (Utilities|Time|PauseTimerbyHandle (Variables|Default|GetTimer)))

(event EventBeginPlay
  (CallFunction|StartTimer))

(fn ConstructionScript)

(fn TimeCalcule
  (if (== (Variables|Default|GetTime_second) 60)
    (Math|Integer|IncrementInt (Variables|Default|GetTime_minute)
      (:%20%20
        (Variables|Default|SetTime_second 0)))
    (else
      (Math|Integer|IncrementInt (Variables|Default|GetTime_second)
        (:%20%20
          _))))
  (return (Utilities|Text|FormatText "{Minutes} : {Secondes}" (Variables|Default|GetTime_minute) (Variables|Default|GetTime_second))))
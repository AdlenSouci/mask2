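; BP_Sound_Controller manages the game's global 2D music and stingers: main theme, fog music, checkpoint and victory sounds.
; BeginPlay pre-creates audio components for each, then starts the main theme.
; Start events spawn a fresh 2D sound component, overwrite the stored reference and play it.
; Pause events, available for all but the checkpoint sound, actually destroy the component, so tracks restart from the beginning rather than resume.
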(event Custom|StartGlobalMusic
  (bind _returnvalue (Audio|CreateSound2D "/Game/Sound_Design/Main_Theme.Main_Theme" 1.0 1.0 0.0 0))
  (bind _output_get (Variables|Default|SetSoundMainTheme _returnvalue))
  (Audio|Components|Audio|Play _output_get 0.0))

(event Custom|PauseGlobalMusic
  (bind _soundmaintheme (Variables|Default|GetSoundMainTheme))
  (Utilities|IsValid _soundmaintheme
    (:Is%20Valid
      (Class|AudioComponent|SetPaused _soundmaintheme true)
      (Components|DestroyComponent _soundmaintheme))))

(event Custom|StartFogMusic
  (bind _returnvalue (Audio|CreateSound2D "/Game/Sound_Design/Music-Fog.Music-Fog" 1.0 1.0 0.0 0))
  (bind _output_get (Variables|Default|SetFogMusic _returnvalue))
  (Audio|Components|Audio|Play _output_get 0.0))

(event Custom|PauseFogMusic
  (bind _fogmusic (Variables|Default|GetFogMusic))
  (Utilities|IsValid _fogmusic
    (:Is%20Valid
      (Class|AudioComponent|SetPaused _fogmusic true)
      (Components|DestroyComponent _fogmusic))))

(event Custom|StartCheckpointSound
  (bind _returnvalue (Audio|CreateSound2D "/Game/Sound_Design/Checkpoint.Checkpoint" 1.0 1.0 0.0 0))
  (bind _output_get (Variables|Default|SetcheckpointMusic _returnvalue))
  (Audio|Components|Audio|Play _output_get 0.0))

(event Custom|StartVictorySound
  (bind _returnvalue (Audio|CreateSound2D "/Game/Sound_Design/Victory.Victory" 1.0 1.0 0.0 0))
  (bind _output_get (Variables|Default|SetVictorySound _returnvalue))
  (Audio|Components|Audio|Play _output_get 0.0))

(event Custom|PauseVictorySound
  (bind _victorysound (Variables|Default|GetVictorySound))
  (Utilities|IsValid _victorysound
    (:Is%20Valid
      (Class|AudioComponent|SetPaused _victorysound true)
      (Components|DestroyComponent _victorysound))))

(event EventBeginPlay
  (bind _returnvalue (Audio|CreateSound2D "/Game/Sound_Design/Victory.Victory" 1.0 1.0 0.0 0))
  (Variables|Default|SetVictorySound _returnvalue)
  (bind _returnvalue_2 (Audio|CreateSound2D "/Game/Sound_Design/Checkpoint.Checkpoint" 1.0 1.0 0.0 0))
  (Variables|Default|SetcheckpointMusic _returnvalue_2)
  (bind _returnvalue_3 (Audio|CreateSound2D "/Game/Sound_Design/Main-theme-final.Main-theme-final" 1.0 1.0 0.0 0))
  (Variables|Default|SetSoundMainTheme _returnvalue_3)
  (bind _returnvalue_4 (Audio|CreateSound2D "/Game/Sound_Design/Music-Fog.Music-Fog" 1.0 1.0 0.0 0))
  (bind _output_get (Variables|Default|SetFogMusic _returnvalue_4))
  (Class|AudioComponent|SetPaused _output_get true)
  (CallFunction|StartGlobalMusic))

(fn ConstructionScript)